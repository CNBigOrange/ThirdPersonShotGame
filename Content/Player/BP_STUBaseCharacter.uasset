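; BP_STUBaseCharacter is a player character Blueprint that toggles custom depth rendering on enemy characters while Q is held.
; Pressing Q finds all actors tagged "Enemy", casts each to this same class and enables Render Custom Depth on its Mesh; releasing Q repeats the search and disables it.
; The file holds no post-process material that uses the depth, and its BeginPlay, overlap, Tick and construction script are empty.
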(event `self.ReceiveBeginPlay`)

(event `self.ReceiveActorBeginOverlap`
  (params (OtherActor :type "Actor Object Reference")))

(event `self.ReceiveTick`
  (params (DeltaSeconds :type "Float (single-precision)")))

(event `Key|Q`
  (params (Key :type "Key Structure"))
  (:`Pressed`
    (bind _outactors (`GameplayStatics.GetAllActorsWithTag` "Enemy"))
    (bind _output_get (set `self.Out Actors` _outactors))
    (for _array_element _output_get
      (bind _asbp_stubase_character (cast `/Game/Player/BP_STUBaseCharacter` _array_element))
      (`PrimitiveComponent.SetRenderCustomDepth` (`Character.Mesh` _asbp_stubase_character) true)))
  (:`Released`
    (bind _outactors_2 (`GameplayStatics.GetAllActorsWithTag` "Enemy"))
    (bind _output_get_2 (set `self.Out Actors` _outactors_2))
    (for _array_element_2 _output_get_2
      (bind _asbp_stubase_character_2 (cast `/Game/Player/BP_STUBaseCharacter` _array_element_2))
      (`PrimitiveComponent.SetRenderCustomDepth` (`Character.Mesh` _asbp_stubase_character_2) false))))

(fn `UserConstructionScript`)